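; Playable Soldier 76 character that sets up health and registers three skills on BeginPlay: sprint, heal and rockets.
; Enhanced Input actions drive the skills: sprint fires while held and finishes on release, heal spawns at the feet, and rockets launch from RocketSpawnPoint.
; Two events swap between regular and ultimate weapons, using timelines to roll both meshes and an event track to toggle visibility and switch weapons mid-animation.
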(event `self.ReceiveBeginPlay`
  (bind _soldier_76_rockets_skill (`self.Soldier_76_Rockets_Skill`))
  (bind _soldier_76_heal_skill (`self.Soldier_76_Heal_Skill`))
  (bind _soldier_76_sprint_skill (`self.Soldier_76_Sprint_Skill`))
  (`parent.ReceiveBeginPlay`)
  (`|ExecutionSequence`
    (:`then_0`
      (`self.InitializeHealth` (make `/Game/_Project/CommonSystems/HealthSystem/HealthData` 250.0 250.0)))
    (:`then_1`
      (`/Game/_Project/CommonSystems/Character_Skills/Character_Skill_BP.Initialize` _soldier_76_sprint_skill self "L SHIFT")
      (`KismetArrayLibrary.Array_Add` (`self.Skills`) _soldier_76_sprint_skill))
    (:`then_2`
      (`/Game/_Project/CommonSystems/Character_Skills/Character_Skill_BP.Initialize` _soldier_76_heal_skill self "E")
      (`KismetArrayLibrary.Array_Add` (`self.Skills`) _soldier_76_heal_skill))
    (:`then_3`
      (`/Game/_Project/CommonSystems/Character_Skills/Character_Skill_BP.Initialize` _soldier_76_rockets_skill self "R CLICK")
      (`KismetArrayLibrary.Array_Add` (`self.Skills`) _soldier_76_rockets_skill))))

(event `EnhancedInput|/Game/_Project/CommonSystems/Input/Skill_0`
  (params (ActionValue :type Boolean) (ElapsedSeconds :type "Float (double-precision)") (TriggeredSeconds :type "Float (double-precision)") (InputAction :type "InputAction Object Reference" :default "/Game/_Project/CommonSystems/Input/Skill_0.Skill_0"))
  (bind _soldier_76_sprint_skill (`self.Soldier_76_Sprint_Skill`))
  (:`Triggered`
    (`/Game/_Project/CommonSystems/Character_Skills/Character_Skill_BP.Fire` _soldier_76_sprint_skill :!label _label))
  (:`Started`
    (goto _label))
  (:`Canceled`
    (`/Game/_Project/CommonSystems/Character_Skills/Character_Skill_BP.Finish` _soldier_76_sprint_skill :!label _label_2))
  (:`Completed`
    (goto _label_2)))

(event `EnhancedInput|/Game/_Project/CommonSystems/Input/Skill_1`
  (params (ActionValue :type Boolean) (ElapsedSeconds :type "Float (double-precision)") (TriggeredSeconds :type "Float (double-precision)") (InputAction :type "InputAction Object Reference" :default "/Game/_Project/CommonSystems/Input/Skill_1.Skill_1"))
  (bind _soldier_76_heal_skill (`self.Soldier_76_Heal_Skill`))
  (:`Started`
    (set `/Game/_Project/Characters/Soldier_76/Skills/Heal/Soldier_76_Heal_Skill.SpawnPoint` (`KismetMathLibrary.Conv_VectorToTransform` (- (`self.K2_GetActorLocation`) (0.0 0.0 85.0))) _soldier_76_heal_skill)
    (`/Game/_Project/CommonSystems/Character_Skills/Character_Skill_BP.Fire` _soldier_76_heal_skill)))

(event `EnhancedInput|/Game/_Project/CommonSystems/Input/SecondaryFire`
  (params (ActionValue :type Boolean) (ElapsedSeconds :type "Float (double-precision)") (TriggeredSeconds :type "Float (double-precision)") (InputAction :type "InputAction Object Reference" :default "/Game/_Project/CommonSystems/Input/SecondaryFire.SecondaryFire"))
  (bind _soldier_76_rockets_skill (`self.Soldier_76_Rockets_Skill`))
  (:`Started`
    (set `/Game/_Project/Characters/Soldier_76/Skills/Rockets/Soldier_76_Rockets_Skill.SpawnPoint` (`SceneComponent.K2_GetComponentToWorld` (`self.RocketSpawnPoint`)) _soldier_76_rockets_skill)
    (`/Game/_Project/CommonSystems/Character_Skills/Character_Skill_BP.Fire` _soldier_76_rockets_skill)))

(event `ChangeToUltimateWeapon`
  (`/Game/_Project/CommonSystems/Weapon/BaseWeapon.Store` (`|GetArrayItem` (`self.Weapons`)))
  (bind (_direction _rotationx) (`Timeline|Timeline` :!via `PlayFromStart`)
    (:`Update`
      (`SceneComponent.K2_SetRelativeRotation` (`self.Mesh`) (`KismetMathLibrary.MakeRotator` _rotationx 0.0 -90.0) false false)
      (`SceneComponent.K2_SetRelativeRotation` (`self.UltimateMesh`) (`KismetMathLibrary.MakeRotator` (+ -1.1 _rotationx) -10.0 -90.0) false false))
    (:`ChangeWeapons`
      (`SceneComponent.SetVisibility` (`self.Mesh`) false false)
      (`SceneComponent.SetVisibility` (`self.UltimateMesh`) true false)
      (`self.ChangeWeapon` 1)
      (`/Game/_Project/CommonSystems/Weapon/BaseWeapon.Draw` (`|GetArrayItem` (`self.Weapons`) 1)))))

(event `ChangeToRegularWeapon`
  (`/Game/_Project/CommonSystems/Weapon/BaseWeapon.Store` (`|GetArrayItem` (`self.Weapons`) 1))
  (bind (_direction _rotationx) (`Timeline|Timeline_0` :!via `PlayFromStart`)
    (:`Update`
      (`SceneComponent.K2_SetRelativeRotation` (`self.Mesh`) (`KismetMathLibrary.MakeRotator` _rotationx 0.0 -90.0) false false)
      (`SceneComponent.K2_SetRelativeRotation` (`self.UltimateMesh`) (`KismetMathLibrary.MakeRotator` (+ -1.1 _rotationx) -10.0 -90.0) false false))
    (:`ChangeWeapons`
      (`SceneComponent.SetVisibility` (`self.Mesh`) true false)
      (`SceneComponent.SetVisibility` (`self.UltimateMesh`) false false)
      (`self.ChangeWeapon` 0)
      (`/Game/_Project/CommonSystems/Weapon/BaseWeapon.Draw` (`|GetArrayItem` (`self.Weapons`))))))

(fn `UserConstructionScript`
  (`parent.UserConstructionScript`))