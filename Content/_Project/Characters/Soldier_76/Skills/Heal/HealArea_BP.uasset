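; Healing area actor for Soldier 76's heal skill that restores health to characters standing inside its sphere.
; Sphere overlap events add and remove HealthSystem components in ActorsInside.
; HealCharacter runs from Tick, and is also bound to a BeginPlay timer, adding typed health scaled by delta seconds to each component.
; A delay inside that loop destroys the area five seconds after it first heals someone.
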(event `self.ReceiveBeginPlay`
  (`KismetSystemLibrary.K2_SetTimerDelegate` (delegate `HealCharacter`) 0.0 true false 0.5))

(event `HealCharacter`
  (bind _result (`BlueprintSetLibrary.Set_ToArray` (`self.ActorsInside`)))
  (for _array_element _result
    (`/Game/_Project/CommonSystems/HealthSystem/HealthSystem.AddHealthType` _array_element (`self.Type`) (* (`self.Heal`) (stale `self.ReceiveTick` DeltaSeconds)))
    (`KismetSystemLibrary.Delay` 5.0)
    (`self.K2_DestroyActor`)))

(event `self.ReceiveTick`
  (params (DeltaSeconds :type "Float (single-precision)"))
  (`self.HealCharacter`))

(event `self.Sphere.OnComponentBeginOverlap`
  (params (OverlappedComponent :type "PrimitiveComponent Object Reference") (OtherActor :type "Actor Object Reference") (OtherComp :type "PrimitiveComponent Object Reference") (OtherBodyIndex :type Integer) (bFromSweep :type Boolean) (SweepResult :type "HitResult Structure (by ref)"))
  (bind _returnvalue (`self.GetComponentByClass` OtherActor "/Game/_Project/CommonSystems/HealthSystem/HealthSystem.HealthSystem_C"))
  (`/Engine/EditorBlueprintResources/StandardMacros.IsValid` _returnvalue
    (:`Is Valid`
      (`BlueprintSetLibrary.Set_Add` (`self.ActorsInside`) _returnvalue))))

(event `self.Sphere.OnComponentEndOverlap`
  (params (OverlappedComponent :type "PrimitiveComponent Object Reference") (OtherActor :type "Actor Object Reference") (OtherComp :type "PrimitiveComponent Object Reference") (OtherBodyIndex :type Integer))
  (bind _returnvalue (`self.GetComponentByClass` OtherActor "/Game/_Project/CommonSystems/HealthSystem/HealthSystem.HealthSystem_C"))
  (`/Engine/EditorBlueprintResources/StandardMacros.IsValid` _returnvalue
    (:`Is Valid`
      (`BlueprintSetLibrary.Set_Remove` (`self.ActorsInside`) _returnvalue))))

(fn `UserConstructionScript`)